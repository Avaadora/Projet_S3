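; Test actor that previews a dissolve effect on a static mesh paired with a Niagara system.
; The construction script creates a dynamic material from slot 0, applies it to slots 0 and 1, and feeds the Amount variable into both material and particles for editor preview.
; On BeginPlay it rebuilds the material the same way and plays the Dissolve timeline, driving the shared Amount parameter from its Alpha track.
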(event EventBeginPlay
  (bind _staticmesh (Variables|Default|GetStaticMesh))
  (bind _returnvalue (Rendering|Material|CreateDynamicMaterialInstance _staticmesh 0 (Rendering|Material|GetMaterial _staticmesh 0) "None" :!class /Script/Engine.PrimitiveComponent))
  (Rendering|Material|SetMaterial _staticmesh 0 _returnvalue)
  (Rendering|Material|SetMaterial _staticmesh 1 _returnvalue)
  (bind _alpha (Timeline|Dissolve PlayFromStart)
    (:Update
      (Rendering|Material|SetScalarParameterValue _returnvalue "Amount" _alpha :!class /Script/Engine.MaterialInstanceDynamic)
      (Effects|Components|ParticleSystem|SetFloatParameter (Variables|Default|GetNiagara) "Amount" _alpha))))

(fn ConstructionScript
  (bind _staticmesh (Variables|Default|GetStaticMesh))
  (bind _returnvalue (Rendering|Material|CreateDynamicMaterialInstance _staticmesh 0 (Rendering|Material|GetMaterial _staticmesh 0) "None" :!class /Script/Engine.PrimitiveComponent))
  (Rendering|Material|SetMaterial _staticmesh 0 _returnvalue)
  (Rendering|Material|SetMaterial _staticmesh 1 _returnvalue)
  (Rendering|Material|SetScalarParameterValue _returnvalue "Amount" (Variables|Default|GetAmount) :!class /Script/Engine.MaterialInstanceDynamic)
  (Effects|Components|ParticleSystem|SetFloatParameter (Variables|Default|GetNiagara) "Amount" (Variables|Default|GetAmount)))