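; Trigger box test actor that burns away a house and animates a statue's material when the Rune actor overlaps it.
; At BeginPlay, each static mesh actor attached to House gets a dynamic dissolve material, an ember Niagara system and a random offset.
; On overlap it resets those pieces, then the Burn timeline drives dissolve, embers and statue Offset, the random values staggering pieces and collision switching off as each fully dissolves.
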(event OnComponentBeginOverlap(Box)
  (params (OverlappedComponent :type Primitive%20Component%20Object%20Reference) (OtherActor :type Actor%20Object%20Reference) (OtherComp :type Primitive%20Component%20Object%20Reference) (OtherBodyIndex :type Integer) (bFromSweep :type Boolean) (SweepResult :type Hit%20Result%20Structure%20%28by%20ref%29))
  (bind _statue (Variables|Default|GetStatue))
  (bind _staticmeshcomponent (Variables|/Script/Engine.StaticMeshActor|GetStaticMeshComponent _statue))
  (if (== OtherActor (Variables|Default|GetRune))
    (CallFunction|CEReset)
    (bind _returnvalue (Rendering|Material|CreateDynamicMaterialInstance _staticmeshcomponent 0 (Rendering|Material|GetMaterial _staticmeshcomponent 0) "None" :!class /Script/Engine.PrimitiveComponent))
    (bind (_direction _house_alpha _embers_alpha _statue_alpha) (Timeline|Burn PlayFromStart)
      (:Update
        (for _array_element (Variables|Default|GetActors)
          (Rendering|Material|SetScalarParameterValue (.material _array_element) "Amount" (Math|Float|Clamp(Float) (- _house_alpha (.materialvalue _array_element))) :!class /Script/Engine.MaterialInstanceDynamic)
          (Effects|Components|ParticleSystem|SetFloatParameter (.niagarasystem _array_element) "Amount" (Math|Float|Clamp(Float) (+ _embers_alpha (.materialvalue _array_element))))
          (Rendering|Material|SetScalarParameterValue _returnvalue "Offset" _statue_alpha :!class /Script/Engine.MaterialInstanceDynamic)
          (if (== (Math|Float|Clamp(Float) (- _house_alpha (.materialvalue _array_element))) 0.0)
            (Collision|SetCollisionEnabled (Variables|/Script/Engine.StaticMeshActor|GetStaticMeshComponent (.staticmesh _array_element)) "NoCollision")))))))

(event Custom|CE_Reset
  (for _array_element (Variables|Default|GetActors)
    (Rendering|Material|SetScalarParameterValue (.material _array_element) "Amount" 1.0 :!class /Script/Engine.MaterialInstanceDynamic)
    (Effects|Components|ParticleSystem|SetFloatParameter (.niagarasystem _array_element) "Amount" 0.0)
    (Collision|SetCollisionEnabled (Variables|/Script/Engine.StaticMeshActor|GetStaticMeshComponent (.staticmesh _array_element)) "QueryAndPhysics")))

(event EventBeginPlay
  (for _array_element (Actor|GetAttachedActors (Variables|Default|GetHouse) true false)
    (bind _asstatic_mesh_actor (Utilities|Casting|CastToStaticMeshActor _array_element))
    (bind _returnvalue (Rendering|Material|CreateDynamicMaterialInstance (Variables|/Script/Engine.StaticMeshActor|GetStaticMeshComponent _asstatic_mesh_actor) 0 (Rendering|Material|GetMaterial (Variables|/Script/Engine.StaticMeshActor|GetStaticMeshComponent _asstatic_mesh_actor) 0) "Dissolve" :!class /Script/Engine.PrimitiveComponent))
    (bind _returnvalue_2 (Niagara|SpawnSystemAttached "/Game/Quentin/TEST/Dissolve/NS_Embers.NS_Embers" (Variables|/Script/Engine.Actor|GetRootComponent _asstatic_mesh_actor) "None" "0, 0, 0" "0, 0, 0" "KeepRelativeOffset" false))
    (Utilities|Array|Add (Variables|Default|GetActors) (Utilities|Struct|MakeS_Actor _asstatic_mesh_actor _returnvalue (Math|Random|RandomFloatinRange 0.0 1.0) _returnvalue_2))))

(fn ConstructionScript)