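; BP_Trigger is a box trigger that receives an active Rune and settles it into a target placement.
; On overlap with its assigned Rune, it makes the first-person player release, freezes the Rune and hides RuneInteraction.
; A timeline then lerps the Rune from its current transform toward RuneLocation and RuneRotation.
; At BeginPlay, it gives a valid Statue a dynamic material instance with its Offset parameter zeroed.
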(event OnComponentBeginOverlap(Box)
  (params (OverlappedComponent :type Primitive%20Component%20Object%20Reference) (OtherActor :type Actor%20Object%20Reference) (OtherComp :type Primitive%20Component%20Object%20Reference) (OtherBodyIndex :type Integer) (bFromSweep :type Boolean) (SweepResult :type Hit%20Result%20Structure%20%28by%20ref%29))
  (bind _rune (Variables|Default|GetRune))
  (bind _rune_2 (Variables|Default|GetRune))
  (if (== OtherActor _rune)
    (if (Variables|/Game/Quentin/Gameplay/Runes/BP_Rune.BP_Rune_C|GetIsActive _rune)
      (bind _asbp_first_person (Utilities|Casting|CastToBP_FirstPerson (Game|Player|GetPlayerPawn 0)))
      (Default|CERelease _asbp_first_person)
      (Default|CEFreeze _rune)
      (Rendering|SetActorHiddenInGame (Variables|Default|GetRune%20Interaction) true)
      (bind _aplha (Timeline|RuneAnimation PlayFromStart)
        (:Update
          (Transformation|SetActorLocationAndRotation _rune_2 (Math|Vector|Lerp(Vector) (Transformation|GetActorLocation _rune_2) (Variables|Default|GetRune%20Location) _aplha) (Math|Rotator|Lerp(Rotator) (Transformation|GetActorRotation _rune_2) (Variables|Default|GetRune%20Rotation) _aplha)))))))

(event EventBeginPlay
  (bind _statue (Variables|Default|GetStatue))
  (bind _staticmeshcomponent (Variables|/Script/Engine.StaticMeshActor|GetStaticMeshComponent _statue))
  (Utilities|IsValid (Variables|Default|GetStatue)
    (:Is%20Valid
      (bind _returnvalue (Rendering|Material|CreateDynamicMaterialInstance (Rendering|Material|GetMaterial _staticmeshcomponent 0) "None" "None" :!class /Script/Engine.KismetMaterialLibrary))
      (Rendering|Material|SetMaterial _staticmeshcomponent 0 _returnvalue)
      (Rendering|Material|SetScalarParameterValue _returnvalue "Offset" 0.0 :!class /Script/Engine.MaterialInstanceDynamic))))

(fn ConstructionScript)