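; BP_Interaction is an interaction point that shows animated prompts and displays a subtitle when activated.
; Its detection sphere, sized from DetectionRadius corrected for scale, pops up a marker in the widget component on player approach.
; External show/hide events swap that marker with an input prompt.
; Activation creates a subtitle widget from Text and blocks prompt changes until deactivation removes it and restores the marker if in range.
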(event OnComponentBeginOverlap(DetectionSphere)
  (params (OverlappedComponent :type Primitive%20Component%20Object%20Reference) (OtherActor :type Actor%20Object%20Reference) (OtherComp :type Primitive%20Component%20Object%20Reference) (OtherBodyIndex :type Integer) (bFromSweep :type Boolean) (SweepResult :type Hit%20Result%20Structure%20%28by%20ref%29))
  (Variables|Default|SetIsPlayerInZone true)
  (if (not (Variables|Default|GetIsPlaying))
    (CallFunction|CEPopUp "Forward")))

(event OnComponentEndOverlap(DetectionSphere)
  (params (OverlappedComponent :type Primitive%20Component%20Object%20Reference) (OtherActor :type Actor%20Object%20Reference) (OtherComp :type Primitive%20Component%20Object%20Reference) (OtherBodyIndex :type Integer))
  (Variables|Default|SetIsPlayerInZone false)
  (if (not (Variables|Default|GetIsPlaying))
    (CallFunction|CEPopUp "Reverse")))

(event Custom|CE_HideInput
  (if (not (Variables|Default|GetIsPlaying))
    (CallFunction|CEPopUpE "Reverse")
    (CallFunction|CEPopUp "Forward")))

(event Custom|CE_Show%20Input
  (if (not (Variables|Default|GetIsPlaying))
    (CallFunction|CEPopUp "Reverse")
    (CallFunction|CEPopUpE "Forward")))

(event Custom|CE_Activate
  (Variables|Default|SetIsPlaying true)
  (CallFunction|CEPopUpE "Reverse")
  (bind _returnvalue (UserInterface|CreateWidget "/Game/Quentin/Gameplay/Interaction/WBP_Subtitle.WBP_Subtitle_C" (Game|GetPlayerController 0)))
  (bind _output_get (Variables|Default|SetWBP_Subtitle _returnvalue))
  (Default|CEUpdateText _output_get (Variables|Default|GetText))
  (UserInterface|Viewport|AddtoViewport _output_get 1)
  (UserInterface|Animation|PlayAnimation _output_get (Variables|/Game/Quentin/Gameplay/Interaction/WBP_Subtitle.WBP_Subtitle_C|GetFade _output_get) 0.0 1 "Forward" 1.0 false))

(event Custom|CE_PopUp
  (params (PlayMode :type EUMGSequencePlayMode%20Enum :default "Forward"))
  (UserInterface|Animation|PlayAnimation (UserInterface|GetWidget (Variables|Default|GetWidget)) (Variables|/Game/Quentin/Gameplay/Interaction/WBP_Interaction.WBP_Interaction_C|GetPopUp (Variables|Default|GetWBP_Interaction)) 0.0 1 PlayMode 1.0 false))

(event Custom|CE_PopUpE
  (params (PlayMode :type EUMGSequencePlayMode%20Enum :default "Forward"))
  (UserInterface|Animation|PlayAnimation (UserInterface|GetWidget (Variables|Default|GetWidget)) (Variables|/Game/Quentin/Gameplay/Interaction/WBP_Interaction.WBP_Interaction_C|GetPopUp_E (Variables|Default|GetWBP_Interaction)) 0.0 1 PlayMode 1.0 false))

(event Custom|CE_Desactivate
  (bind _wbp_subtitle (Variables|Default|GetWBP_Subtitle))
  (UserInterface|Animation|PlayAnimation _wbp_subtitle (Variables|/Game/Quentin/Gameplay/Interaction/WBP_Subtitle.WBP_Subtitle_C|GetFade _wbp_subtitle) 0.0 1 "Reverse" 1.0 false)
  (Widget|RemovefromParent _wbp_subtitle)
  (Variables|Default|SetIsPlaying false)
  (if (Variables|Default|GetIsPlayerInZone)
    (CallFunction|CEPopUp "Forward")))

(event EventBeginPlay
  (Rendering|Material|SetMaterial (Variables|Default|GetCenter) 0 "/Game/Quentin/Gameplay/Interaction/M_Invisible.M_Invisible")
  (bind _aswbp_interaction (Utilities|Casting|CastToWBP_Interaction (UserInterface|GetWidget (Variables|Default|GetWidget))))
  (Variables|Default|SetWBP_Interaction _aswbp_interaction))

(fn ConstructionScript
  (Components|Sphere|SetSphereRadius (Variables|Default|GetDetectionSphere) (/ (Variables|Default|GetDetection%20Radius) (.x (Transformation|GetWorldScale (Variables|Default|GetCenter)))) true))