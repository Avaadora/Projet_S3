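; BP_DecalRune is a placeable decal actor that shows a configurable rune on surfaces.
; Its construction script creates a dynamic instance of the decal material and feeds it the rune texture, color, intensity and wave toggle.
; Each construction also rolls a random wave parameter to vary runes.
; The editor billboard's screen size is divided by the actor's X scale, with a cap, to offset scaling.
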(fn ConstructionScript
  (bind _returnvalue (Rendering|Material|CreateDynamicMaterialInstance (Class|DecalComponent|GetDecalMaterial (Variables|Default|GetDecal)) "None" "None" :!class /Script/Engine.KismetMaterialLibrary))
  (Rendering|Material|SetTextureParameterValue _returnvalue "Rune Texture" (Variables|Default|GetTexture))
  (Rendering|Material|SetVectorParameterValue _returnvalue "Rune Color" (Variables|Default|GetColor) :!class /Script/Engine.MaterialInstanceDynamic)
  (Rendering|Material|SetScalarParameterValue _returnvalue "Rune Intensity" (Variables|Default|GetIntensity) :!class /Script/Engine.MaterialInstanceDynamic)
  (Rendering|Material|SetScalarParameterValue _returnvalue "Use Wave" (Math|Conversions|ToFloat(Integer) (Variables|Default|GetUseWave)) :!class /Script/Engine.MaterialInstanceDynamic)
  (Rendering|Material|SetScalarParameterValue _returnvalue "Rune Wave" (Math|Random|RandomFloatinRange 1.0 5.0) :!class /Script/Engine.MaterialInstanceDynamic)
  (Rendering|Components|Decal|SetDecalMaterial (Variables|Default|GetDecal) _returnvalue)
  (Variables|/Script/Engine.BillboardComponent|SetScreenSize (Variables|Default|GetDecalBilboard) (Math|Float|Clamp(Float) (/ (Math|Float|MakeLiteralFloat 0.0005) (.x (Class|Actor|GetActorRelativeScale3D))) 0.0 0.0005)))