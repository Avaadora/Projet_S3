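; BP_Rune is a rune actor with a configurable mesh and a scale-compensated detection sphere that drives an interaction prompt widget.
; Entering or leaving the sphere plays the widget's pop-up animation forward or in reverse.
; Show and hide input events swap it with a left-click prompt while the rune is inactive.
; Activate and deactivate update that state, and freeze disables physics and collision and destroys the widget.
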(event OnComponentBeginOverlap(DetectionSphere)
  (params (OverlappedComponent :type Primitive%20Component%20Object%20Reference) (OtherActor :type Actor%20Object%20Reference) (OtherComp :type Primitive%20Component%20Object%20Reference) (OtherBodyIndex :type Integer) (bFromSweep :type Boolean) (SweepResult :type Hit%20Result%20Structure%20%28by%20ref%29))
  (CallFunction|CEPopUp "Forward"))

(event OnComponentEndOverlap(DetectionSphere)
  (params (OverlappedComponent :type Primitive%20Component%20Object%20Reference) (OtherActor :type Actor%20Object%20Reference) (OtherComp :type Primitive%20Component%20Object%20Reference) (OtherBodyIndex :type Integer))
  (CallFunction|CEPopUp "Reverse"))

(event Custom|CE_HideInput
  (if (not (Variables|Default|GetIsActive))
    (CallFunction|CEPopUpLeftClick "Reverse")
    (CallFunction|CEPopUp "Forward")))

(event Custom|CE_ShowInput
  (if (not (Variables|Default|GetIsActive))
    (CallFunction|CEPopUp "Reverse")
    (CallFunction|CEPopUpLeftClick "Forward")))

(event Custom|CE_PopUp
  (params (PlayMode :type EUMGSequencePlayMode%20Enum :default "Forward"))
  (Utilities|IsValid (Variables|Default|GetWidget)
    (:Is%20Valid
      (UserInterface|Animation|PlayAnimation (UserInterface|GetWidget (Variables|Default|GetWidget)) (Variables|/Game/Quentin/Gameplay/Interaction/WBP_Interaction.WBP_Interaction_C|GetPopUp (Variables|Default|GetWBP_Interaction)) 0.0 1 PlayMode 1.0 false))))

(event Custom|CE_PopUpLeftClick
  (params (PlayMode :type EUMGSequencePlayMode%20Enum :default "Forward"))
  (Utilities|IsValid (Variables|Default|GetWidget)
    (:Is%20Valid
      (UserInterface|Animation|PlayAnimation (UserInterface|GetWidget (Variables|Default|GetWidget)) (Variables|/Game/Quentin/Gameplay/Interaction/WBP_Interaction.WBP_Interaction_C|GetPopUp_LeftClick (Variables|Default|GetWBP_Interaction)) 0.0 1 PlayMode 1.0 false))))

(event Custom|CE_Desactivate
  (Variables|Default|SetIsActive false)
  (CallFunction|CEPopUp "Forward"))

(event Custom|CE_Activate
  (Variables|Default|SetIsActive true)
  (CallFunction|CEPopUpLeftClick "Reverse"))

(event Custom|CE_Freeze
  (bind _mesh (Variables|Default|GetMesh))
  (Physics|SetSimulatePhysics _mesh false)
  (Collision|SetCollisionEnabled _mesh "NoCollision")
  (Components|DestroyComponent (Variables|Default|GetWidget)))

(event EventBeginPlay
  (bind _aswbp_interaction (Utilities|Casting|CastToWBP_Interaction (UserInterface|GetWidget (Variables|Default|GetWidget))))
  (Variables|Default|SetWBP_Interaction _aswbp_interaction))

(fn ConstructionScript
  (Components|Sphere|SetSphereRadius (Variables|Default|GetDetectionSphere) (/ (Variables|Default|GetDetection%20Radius) (.x (Transformation|GetWorldScale (Variables|Default|GetMesh)))) true)
  (Components|StaticMesh|SetStaticMesh (Variables|Default|GetMesh) (Variables|Default|GetRuneMesh)))