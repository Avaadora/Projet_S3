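; BP_Rune is a rune actor with a configurable mesh and an interaction prompt widget driven by player proximity.
; An outer detection sphere plays the widget's PopUp animation on overlap and reverses it on exit.
; An inner interaction sphere swaps PopUp for the PopUpE prompt on entry and back on exit, with no overlap filtering or interaction logic here.
; The construction script applies the RuneMesh variable to the mesh component.
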(event OnComponentBeginOverlap(DetectionSphere)
  (params (OverlappedComponent :type Primitive%20Component%20Object%20Reference) (OtherActor :type Actor%20Object%20Reference) (OtherComp :type Primitive%20Component%20Object%20Reference) (OtherBodyIndex :type Integer) (bFromSweep :type Boolean) (SweepResult :type Hit%20Result%20Structure%20%28by%20ref%29))
  (UserInterface|Animation|PlayAnimation (UserInterface|GetWidget (Variables|Default|GetWidget)) (Variables|/Game/Quentin/Gameplay/WBP_Interaction.WBP_Interaction_C|GetPopUp (Variables|Default|GetWBP_Interaction)) 0.0 1 "Forward" 1.0 false))

(event OnComponentEndOverlap(DetectionSphere)
  (params (OverlappedComponent :type Primitive%20Component%20Object%20Reference) (OtherActor :type Actor%20Object%20Reference) (OtherComp :type Primitive%20Component%20Object%20Reference) (OtherBodyIndex :type Integer))
  (UserInterface|Animation|PlayAnimation (UserInterface|GetWidget (Variables|Default|GetWidget)) (Variables|/Game/Quentin/Gameplay/WBP_Interaction.WBP_Interaction_C|GetPopUp (Variables|Default|GetWBP_Interaction)) 0.0 1 "Reverse" 1.0 false))

(event OnComponentBeginOverlap(InteractionSphere)
  (params (OverlappedComponent :type Primitive%20Component%20Object%20Reference) (OtherActor :type Actor%20Object%20Reference) (OtherComp :type Primitive%20Component%20Object%20Reference) (OtherBodyIndex :type Integer) (bFromSweep :type Boolean) (SweepResult :type Hit%20Result%20Structure%20%28by%20ref%29))
  (UserInterface|Animation|PlayAnimation (UserInterface|GetWidget (Variables|Default|GetWidget)) (Variables|/Game/Quentin/Gameplay/WBP_Interaction.WBP_Interaction_C|GetPopUp (Variables|Default|GetWBP_Interaction)) 0.0 1 "Reverse" 1.0 false)
  (UserInterface|Animation|PlayAnimation (UserInterface|GetWidget (Variables|Default|GetWidget)) (Variables|/Game/Quentin/Gameplay/WBP_Interaction.WBP_Interaction_C|GetPopUp_E (Variables|Default|GetWBP_Interaction)) 0.0 1 "Forward" 1.0 false))

(event OnComponentEndOverlap(InteractionSphere)
  (params (OverlappedComponent :type Primitive%20Component%20Object%20Reference) (OtherActor :type Actor%20Object%20Reference) (OtherComp :type Primitive%20Component%20Object%20Reference) (OtherBodyIndex :type Integer))
  (UserInterface|Animation|PlayAnimation (UserInterface|GetWidget (Variables|Default|GetWidget)) (Variables|/Game/Quentin/Gameplay/WBP_Interaction.WBP_Interaction_C|GetPopUp_E (Variables|Default|GetWBP_Interaction)) 0.0 1 "Reverse" 1.0 false)
  (UserInterface|Animation|PlayAnimation (UserInterface|GetWidget (Variables|Default|GetWidget)) (Variables|/Game/Quentin/Gameplay/WBP_Interaction.WBP_Interaction_C|GetPopUp (Variables|Default|GetWBP_Interaction)) 0.0 1 "Forward" 1.0 false))

(event EventBeginPlay
  (bind _aswbp_interaction (Utilities|Casting|CastToWBP_Interaction (UserInterface|GetWidget (Variables|Default|GetWidget))))
  (Variables|Default|SetWBP_Interaction _aswbp_interaction))

(fn ConstructionScript
  (Components|StaticMesh|SetStaticMesh (Variables|Default|GetRune) (Variables|Default|GetRuneMesh)))