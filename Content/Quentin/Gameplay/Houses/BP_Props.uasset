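; BP_Props manages attached static mesh actors as props that can burn away, dissolving with embers before being removed.
; BeginPlay gives each mesh dynamic materials and a random offset, stored in a Props array.
; CE_Burn attaches an ember Niagara system to each, then a timeline drives the "Amount" parameter on materials and particles, staggered by that offset.
; When finished, it disables collision, makes slot 0 invisible and destroys the attached actors.
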(event Custom|CE_Burn
  (for (_array_element _array_index) (Variables|Default|GetProps)
    (bind _returnvalue (Niagara|SpawnSystemAttached "/Game/Quentin/Gameplay/Houses/NS_Embers.NS_Embers" (.mesh _array_element) "None" "0, 0, 0" "0, 0, 0" "KeepRelativeOffset" false))
    (Utilities|Array|SetArrayElem (Variables|Default|GetProps) _array_index (Utilities|Struct|MakeS_Props (.mesh _array_element) (.materials _array_element) (.materialvalue _array_element) _returnvalue))
    (bind _alpha (Timeline|Timeline PlayFromStart)
      (:Update
        (for _array_element_2 (Variables|Default|GetProps)
          (Effects|Components|ParticleSystem|SetFloatParameter (.niagarasystem _array_element_2) "Amount" (- (* _alpha 2.0) (.materialvalue _array_element_2)))
          (for _array_element_3 (.materials _array_element_2)
            (Rendering|Material|SetScalarParameterValue _array_element_3 "Amount" (- (* _alpha 2.0) (.materialvalue _array_element_2)) :!class /Script/Engine.MaterialInstanceDynamic))))
      (:Finished
        (for _array_element_4 (Variables|Default|GetProps)
          (Collision|SetCollisionEnabled (.mesh _array_element_4) "NoCollision")
          (Rendering|Material|SetMaterial (.mesh _array_element_4) 0 "/Game/Quentin/Gameplay/Interaction/M_Invisible.M_Invisible"))
        (for _array_element_5 (Actor|GetAttachedActors true false)
          (Actor|DestroyActor _array_element_5))))))

(event EventBeginPlay
  (for _array_element (Actor|GetAttachedActors true false)
    (bind _asstatic_mesh_actor (Utilities|Casting|CastToStaticMeshActor _array_element))
    (Utilities|Array|Clear (Variables|Default|GetMaterials))
    (for _index (range 0 (- (Rendering|Material|GetNumMaterials (Variables|/Script/Engine.StaticMeshActor|GetStaticMeshComponent _asstatic_mesh_actor)) 1))
      (bind _returnvalue (Rendering|Material|CreateDynamicMaterialInstance (Rendering|Material|GetMaterial (Variables|/Script/Engine.StaticMeshActor|GetStaticMeshComponent _asstatic_mesh_actor) _index) "None" "None" :!class /Script/Engine.KismetMaterialLibrary))
      (Rendering|Material|SetMaterial (Variables|/Script/Engine.StaticMeshActor|GetStaticMeshComponent _asstatic_mesh_actor) _index _returnvalue)
      (Utilities|Array|Add (Variables|Default|GetMaterials) _returnvalue))
    (Utilities|Array|Add (Variables|Default|GetProps) (Utilities|Struct|MakeS_Props (Variables|/Script/Engine.StaticMeshActor|GetStaticMeshComponent _asstatic_mesh_actor) (Variables|Default|GetMaterials) (Math|Random|RandomFloatinRange 0.0 1.0) 0))))

(fn ConstructionScript)