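; Raven sound actor that repeatedly plays a shortened raven audio clip at random intervals.
; BeginPlay assigns the clip to the Audio component and starts a custom event that waits a few seconds before the first play.
; The event then loops endlessly through play and a random delay between MinTime and MaxTime.
; A delayed Stop branch exists but never runs.
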(event Custom|CE_PlaySound
  (Utilities|FlowControl|Delay 4.0)
  (Audio|Components|Audio|Play (Variables|Default|GetAudio) 0.0 :!label _label)
  (Utilities|FlowControl|Delay (Math|Random|RandomFloatinRange (Variables|Default|GetMinTime) (Variables|Default|GetMaxTime)))
  (goto _label))

(event EventBeginPlay
  (Audio|Components|Audio|SetSound (Variables|Default|GetAudio) "/Game/Manon/Audio/A_Raven_Shorten.A_Raven_Shorten")
  (CallFunction|CEPlaySound))

(fn ConstructionScript)